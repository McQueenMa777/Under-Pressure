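; Click-to-move player character in a fish-seeking game with a countdown meter.
; Left click traces under the cursor, runs SimpleMoveToLocation, drops a short-lived marker and sets facing from the X direction.
; Tick scales bubble Niagara parameters by speed and points an arrow at the nearest fish.
; When the meter UI's countdown hits zero, it explodes once, hiding the mesh and bubbles, disabling collision and destroying the arrow.
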(event Custom|NavigateToNearestFish
  (bind _returnvalue (Transformation|GetActorLocation))
  ;[1 1 1] ArrowNavigation
  (bind _outactors (Actor|GetAllActorsOfClass "/Game/FishActorClass.FishActorClass_C"))
  (Transformation|SetWorldRotation (Variables|Default|GetArrowBase) (Math|Rotator|MakeRotfromXZ (Math|Vector|Normalize (- (Transformation|GetActorLocation (.ReturnValue (Actor|FindNearestActor _returnvalue _outactors))) _returnvalue)) (Math|Vector|MakeVector 0.0 0.0 -1.0)) false false))

(event Custom|GameOver
  ;[1 1 1] GameOver
  (Niagara|SpawnSystematLocation "/Game/ExplosionNiagara.ExplosionNiagara" (Transformation|GetWorldLocation (Variables|Collision|GetCapsuleComponent)))
  (Variables|Default|SetExplosionSpawned? true)
  (Rendering|SetVisibility (Variables|Default|Getbubbles) false false)
  (Collision|SetCollisionEnabled (Variables|Collision|GetCapsuleComponent) "NoCollision")
  (Rendering|SetVisibility (Variables|Default|GetSkeletalMesh) false false)
  (Audio|SpawnSound2D "/Game/Audio/explode.explode" 1.0 1.0 0.0 0)
  (Components|DestroyComponent (Variables|Default|GetUIArrow)))

(event EventBeginPlay
  ;[1 1 1] InitialSettings
  (Variables|/Script/Engine.PlayerController|SetbShowMouseCursor (Game|GetPlayerController 0) true)
  (bind _returnvalue (UserInterface|CreateWidget "/Game/BP_UI/BP_MeterUI.BP_MeterUI_C"))
  (bind _output_get (Variables|Default|SetMeterUI _returnvalue))
  (UserInterface|Viewport|AddtoViewport _output_get 0)
  (Default|PlayBeep (CallFunction|GetGameManager))
  (bind _returnvalue_2 (AddComponent|AddAudioComponent false))
  (Variables|Default|SetBGM _returnvalue_2))

(event EventTick
  (params (DeltaSeconds :type Float%20%28single-precision%29))
  (bind _returnvalue (Transformation|GetVelocity))
  (bind _returnvalue_2 (Math|Vector|VectorLength _returnvalue))
  ;[1 1 1] Set Niagara
  (Class|NiagaraComponent|SetVariableInt (Variables|Default|Getbubbles) "UserSpawnRate" (Math|Float|Truncate (Math|Float|MapRangeClamped _returnvalue_2 0.0 6e+02 0.0 2e+01)))
  (Class|NiagaraComponent|SetVariableInt (Variables|Default|Getbubbles) "ParticleVelocity" (Math|Float|Truncate (/ _returnvalue_2 2e+01)))
  (Variables|Default|SetYlocation (.y (Transformation|GetWorldLocation (Variables|Collision|GetCapsuleComponent))))
  ;[1 1 1] GameOverCheck
  (if (== (Variables|/Game/BP_UI/BP_MeterUI.BP_MeterUI_C|GetCountdownNumber (Variables|Default|GetMeterUI)) 0.0)
    (if (not (Variables|Default|GetExplosionSpawned?))
      (CallFunction|GameOver))
    (else
      (CallFunction|NavigatetoNearestFish))))

(event Input|MouseEvents|LeftMouseButton
  (params (Key :type Key%20Structure :default "None"))
  (bind _returnvalue (Game|GetPlayerController 0))
  (bind _base (Variables|Default|GetBase))
  (bind (_worldlocation _worlddirection) (Game|Player|ConvertMouseLocationToWorldSpace _returnvalue))
  ;[1 1 1] Line Trace
  (:Pressed
    (bind (_outhit _returnvalue_2) (Collision|LineTraceByChannel _worldlocation (+ _worldlocation (* _worlddirection 5e+03)) "TraceTypeQuery1" false 0 "None" true "(R=1.000000,G=0.000000,B=0.000000,A=1.000000)" "(R=0.000000,G=1.000000,B=0.000000,A=1.000000)" 2.0))
    ;[1 1 1] Move
    (if _returnvalue_2
      (AI|Navigation|SimpleMovetoLocation (Game|GetPlayerController 0) (.Location (Collision|BreakHitResult _outhit)))
      ;[1 1 1] Cursor Spawning
      (Utilities|IsValid (Variables|Default|Getcursor)
        (:Is%20Valid
          (Actor|DestroyActor (Variables|Default|Getcursor)))
        (:Is%20Not%20Valid
          _))
      (bind _returnvalue_3 (Game|SpawnActorfromClass "/Game/BP_Cursor/BP_Cursor.BP_Cursor_C" (Math|Transform|MakeTransform (.Location (Collision|BreakHitResult _outhit)) "0, 0, 0" "10.000000,10.000000,10.000000") "Undefined" 0 0))
      (Actor|SetLifeSpan _returnvalue_3 1.2)
      (Variables|Default|Setcursor _returnvalue_3)
      ;[1 1 1] Turning?
      (if (< (.x (- (.Location (Collision|BreakHitResult _outhit)) (Transformation|GetActorLocation))) 0.0)
        (Transformation|SetWorldRotation _base (Math|Rotator|MakeRotfromXY (Math|Vector|MakeVector -1.0 0.0 0.0) (Math|Vector|MakeVector 0.0 1.0 0.0)) false false)
        (else
          (Transformation|SetWorldRotation _base (Class|KismetMathLibrary|MakeRotfromYX (Math|Vector|MakeVector 0.0 0.0 0.0) (Math|Vector|MakeVector 0.0 0.0 0.0)) false false))))))

(fn ConstructionScript)