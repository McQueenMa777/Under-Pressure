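; BP_GameManager is a game manager that fades full-screen post-process effects, starts a beep sound and toggles UI visibility.
; On BeginPlay it caches the dark blue, black and hell post-process components from MainChar.
; Each fade event plays or reverses its own timeline to drive that component's blend weight.
; PlayBeep stores a newly added audio component, and SetUIVisibility shows or hides a given widget from the IsUIVisible flag.
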(event Custom|FadeHellPostProcess
  (params (In :type Boolean))
  (if In
    (bind _change_in_blend_weight (Timeline|Timeline_1 Play)
      (:Update
        (Variables|/Script/Engine.PostProcessComponent|SetBlendWeight (Variables|Default|GetHellPostProcess) _change_in_blend_weight)))
    (else
      (Timeline|Timeline_1 Reverse))))

(event Custom|FadeDarkBluePostprocess
  (params (In :type Boolean))
  ;[1 1 1] Fade Dark Blue
  (if In
    (bind _change_in_blend_weight (Timeline|Timeline Play)
      (:Update
        (Variables|/Script/Engine.PostProcessComponent|SetBlendWeight (Variables|Default|GetDarkBluePostProcess) _change_in_blend_weight)))
    (else
      (Timeline|Timeline Reverse))))

(event Custom|PlayBeep
  (bind _returnvalue (AddComponent|AddAudioComponent false))
  (Variables|Default|SetBeepSound _returnvalue))

(event Custom|FadeBlackPostProcess
  (params (In :type Boolean))
  (if In
    (bind _change_in_blend_weight (Timeline|Timeline_0 Play)
      (:Update
        (Variables|/Script/Engine.PostProcessComponent|SetBlendWeight (Variables|Default|GetBlackPostProcess) _change_in_blend_weight)))
    (else
      (Timeline|Timeline_0 Reverse))))

(event EventBeginPlay
  ;[1 1 1] Set Post Processes Component
  (Variables|Default|SetDarkBluePostProcess (Variables|/Game/BP_Character.BP_Character_C|GetPostProcessDarkBlue (Variables|Default|GetMainChar)))
  (Variables|Default|SetBlackPostProcess (Variables|/Game/BP_Character.BP_Character_C|GetPostProcessBlack (Variables|Default|GetMainChar)))
  (Variables|Default|SetHellPostProcess (Variables|/Game/BP_Character.BP_Character_C|GetPostProcessHell (Variables|Default|GetMainChar))))

(fn ConstructionScript)

(fn SetUIVisibility
  (params (WindowUI :type BP%20Window%20UI%20Object%20Reference))
  (if (Variables|Default|GetIsUIVisible)
    (Widget|SetVisibility WindowUI "Visible")
    (else
      (Widget|SetVisibility WindowUI "Hidden"))))