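; Test fish actor that travels a relative path and opens a name-specific popup when touched.
; InterpToMovement gets control points at its origin and MoveTo, added in both the construction script and BeginPlay.
; On overlap it creates BP_WindowUI with FishName, switches to UI-only input, registers the window with the game manager, then destroys itself.
; Destruction makes an image on the main character's meter UI visible.
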(event OnComponentBeginOverlap(Collision)
  (params (OverlappedComponent :type Primitive%20Component%20Object%20Reference) (OtherActor :type Actor%20Object%20Reference) (OtherComp :type Primitive%20Component%20Object%20Reference) (OtherBodyIndex :type Integer) (bFromSweep :type Boolean) (SweepResult :type Hit%20Result%20Structure%20%28by%20ref%29))
  (bind _man (CallFunction|GetGameManager))
  (bind _returnvalue (UserInterface|CreateWidget "/Game/BP_UI/BP_WindowUI.BP_WindowUI_C"))
  (bind _output_get (Variables|Default|SetWindowUI _returnvalue))
  (Variables|/Game/BP_UI/BP_WindowUI.BP_WindowUI_C|SetFishName _output_get (Variables|Default|GetFishName))
  (UserInterface|Viewport|AddtoViewport _output_get 0)
  (Input|SetInputModeUIOnly (Game|GetPlayerController 0) 0 "DoNotLock" false)
  (Default|CheckFishNameandPlayPopOut (Variables|Default|GetWindowUI))
  (UserInterface|Animation|PlayAnimation (Variables|Default|GetWindowUI) (Variables|/Game/BP_UI/BP_WindowUI.BP_WindowUI_C|GetFadeIn (Variables|Default|GetWindowUI)) 0.0 1 "Forward" 1.0 false)
  (Variables|/Game/BP_General/BP_GameManager.BP_GameManager_C|SetIsUIVisible _man true)
  (Default|SetUIVisibility _man (Variables|Default|GetWindowUI))
  (Actor|DestroyActor))

(event EventBeginPlay
  (Class|InterptoMovementComponent|AddControlPointPosition (Variables|Default|GetInterpToMovement) "0, 0, 0" true)
  (Class|InterptoMovementComponent|AddControlPointPosition (Variables|Default|GetInterpToMovement) (Variables|Default|GetMoveTo) true))

(event EventDestroyed
  (bind _maincharacter (CallFunction|GetMainCharacter))
  (Widget|SetVisibility (Variables|/Game/BP_UI/BP_MeterUI.BP_MeterUI_C|GetImage_0 (Variables|/Game/BP_Character.BP_Character_C|GetMeterUI _maincharacter)) "Visible"))

(fn ConstructionScript
  (Development|PrintString "Hello")
  (Class|InterptoMovementComponent|AddControlPointPosition (Variables|Default|GetInterpToMovement) "0, 0, 0" true)
  (Class|InterptoMovementComponent|AddControlPointPosition (Variables|Default|GetInterpToMovement) (Variables|Default|GetMoveTo) true))