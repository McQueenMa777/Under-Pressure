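; BP_Hellbass is a collectible Hellbass fish that patrols back and forth and opens a fish info window on overlap.
; Its InterpToMovement reversals toggle a Turn flag to flip the base mesh's facing.
; Overlap shows a BP_WindowUI with the fish name, plays bubbling audio, registers the UI with the game manager, destroys the fish and pauses.
; On destruction it ticks the Hellfish checkbox on the main character's meter UI.
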(event OnInterptoReverse(InterpToMovement)
  (params (ImpactResult :type Hit%20Result%20Structure%20%28by%20ref%29) (Time :type Float%20%28single-precision%29))
  (bind _base (Variables|Default|GetBase))
  (if (Variables|Default|GetTurn?)
    (Transformation|SetWorldRotation _base (Math|Rotator|MakeRotfromXZ (Math|Vector|MakeVector 1.0 0.0 0.0) (Math|Vector|MakeVector 0.0 -1.0 0.0)) false false)
    (Variables|Default|SetTurn? false)
    (else
      (Transformation|SetWorldRotation _base (Math|Rotator|MakeRotfromXZ (Math|Vector|MakeVector -1.0 0.0 0.0) (Math|Vector|MakeVector 0.0 -1.0 0.0)) false false)
      (Variables|Default|SetTurn? true))))

(event EventBeginPlay
  (Transformation|SetWorldRotation (Variables|Default|GetBase) (Math|Rotator|MakeRotfromXZ (Math|Vector|MakeVector 1.0 0.0 0.0) (Math|Vector|MakeVector 0.0 -1.0 0.0)) false false))

(event EventDestroyed
  (bind _maincharacter (CallFunction|GetMainCharacter))
  (Class|CheckBox|SetCheckedState (Variables|/Game/BP_UI/BP_MeterUI.BP_MeterUI_C|GetHellfishCheckBox (Variables|/Game/BP_Character.BP_Character_C|GetMeterUI _maincharacter)) "Checked"))

(event Collision|EventActorBeginOverlap
  (params (OtherActor :type Actor%20Object%20Reference))
  (bind _man (CallFunction|GetGameManager))
  (bind _returnvalue (UserInterface|CreateWidget "/Game/BP_UI/BP_WindowUI.BP_WindowUI_C"))
  (bind _output_get (Variables|Default|SetWindowUI _returnvalue))
  (Variables|/Game/BP_UI/BP_WindowUI.BP_WindowUI_C|SetFishName _output_get (Variables|Default|GetFishName))
  (UserInterface|Viewport|AddtoViewport _output_get 0)
  (Input|SetInputModeUIOnly (Game|GetPlayerController 0) 0 "DoNotLock" false)
  (Default|CheckFishNameandPlayPopOut (Variables|Default|GetWindowUI))
  (UserInterface|Animation|PlayAnimation (Variables|Default|GetWindowUI) (Variables|/Game/BP_UI/BP_WindowUI.BP_WindowUI_C|GetFadeIn (Variables|Default|GetWindowUI)) 0.0 1 "Forward" 1.0 false)
  (Audio|PlaySound2D "/Game/Audio/BubblingSound.BubblingSound" 1.0 1.0 0.0 0 0)
  (Variables|/Game/BP_General/BP_GameManager.BP_GameManager_C|SetIsUIVisible _man true)
  (Default|SetUIVisibility _man (Variables|Default|GetWindowUI))
  (Actor|DestroyActor)
  (Game|SetGamePaused true))

(fn ConstructionScript
  (|CallParentFunction))